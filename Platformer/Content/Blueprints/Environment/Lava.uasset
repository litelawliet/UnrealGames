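; Lava hazard actor that damages the player character while it stands inside it.
; On begin play it spawns a looping lava sound at its location with distance attenuation.
; Overlap begin and end with a ThirdPersonCharacter toggle a Damaging flag.
; While the flag is set, Tick subtracts DamageValue from player zero's CurrentHealth every frame, so damage depends on frame rate.
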(event `self.ReceiveBeginPlay`
  (`GameplayStatics.SpawnSoundAtLocation` "/Game/Assets/Sounds/lava-loop.lava-loop" (`self.K2_GetActorLocation`) (struct) 4.0 1.0 0.0 "/Game/Assets/Sounds/LavaSoundAttenuation.LavaSoundAttenuation" null))

(event `self.ReceiveActorBeginOverlap`
  (params (OtherActor :type "Actor Object Reference"))
  (cast `/Game/ThirdPersonBP/Blueprints/ThirdPersonCharacter` OtherActor)
  (set `self.Damaging` true))

(event `self.ReceiveActorEndOverlap`
  (params (OtherActor :type "Actor Object Reference"))
  (cast `/Game/ThirdPersonBP/Blueprints/ThirdPersonCharacter` OtherActor)
  (set `self.Damaging` false))

(event `self.ReceiveTick`
  (params (DeltaSeconds :type "Float (single-precision)"))
  (`self.DamagePlayer`))

(fn `DamagePlayer`
  (if (`self.Damaging`)
    (bind _asthird_person_character (cast `/Game/ThirdPersonBP/Blueprints/ThirdPersonCharacter` (`GameplayStatics.GetPlayerCharacter` 0)))
    (set `/Game/ThirdPersonBP/Blueprints/ThirdPersonCharacter.CurrentHealth` (- (`/Game/ThirdPersonBP/Blueprints/ThirdPersonCharacter.CurrentHealth` _asthird_person_character) (`self.DamageValue`)) _asthird_person_character)))

(fn `UserConstructionScript`)
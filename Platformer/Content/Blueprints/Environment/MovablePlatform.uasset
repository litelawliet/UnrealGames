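; Moving platform actor that oscillates back and forth around its starting location along any combination of X, Y and Z.
; BeginPlay stores the origin, and Tick accumulates time and sets the location from ComputeNewVector without sweeping.
; ComputeNewVector applies Range to each enabled Axis flag and lerps by the sine of time, so motion swings to both sides of the origin.
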(event `self.ReceiveBeginPlay`
  (set `self.Origin` (`self.K2_GetActorLocation`)))

(event `self.ReceiveTick`
  (params (DeltaSeconds :type "Float (single-precision)"))
  (bind _result (`self.ComputeNewVector`))
  (`self.K2_SetActorLocation` _result)
  (set `self.time` (+ (`self.time`) DeltaSeconds)))

(fn `ComputeNewVector`
  (returns (Result :type "Vector Structure"))
  (bind _axis (`self.axis`))
  (bind _returnvalue (`KismetMathLibrary.Conv_IntToDouble` (`self.Range`)))
  ;[1 1 1] Move the plateform accordingly of the axis
  (if (`|GetArrayItem` _axis)
    (bind _output_get (set `self.tempX` _returnvalue)))
  (if (`|GetArrayItem` _axis 1)
    (bind _output_get_2 (set `self.tempY` _returnvalue)))
  (if (`|GetArrayItem` _axis 2)
    (bind _output_get_3 (set `self.tempZ` _returnvalue)))
  (return (`KismetMathLibrary.VLerp` (`self.Origin`) (+ (`self.Origin`) (`KismetMathLibrary.MakeVector` _output_get _output_get_2 _output_get_3)) (`KismetMathLibrary.Sin` (`self.time`)))))

(fn `UserConstructionScript`)
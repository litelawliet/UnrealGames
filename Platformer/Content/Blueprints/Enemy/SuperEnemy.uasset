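; SuperEnemy is an enemy Blueprint that retreats to its starting point to recover when down to one life.
; It records that point shortly after BeginPlay, and Tick runs CheckHealth, which sets the retreat state at one life.
; Tick then issues AIMoveTo and checks arrival by position, using a flag to block repeats.
; On arrival it plays a collapse sound, waits, regains a life and restores its initial state.
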(event `self.ReceiveBeginPlay`
  (`parent.ReceiveBeginPlay`)
  (`KismetSystemLibrary.Delay` 2.0)
  (set `self.StartingPoint` (`self.K2_GetActorLocation`)))

(event `self.ReceiveTick`
  (params (DeltaSeconds :type "Float (single-precision)"))
  (bind (_returnvalue_x _returnvalue_y _returnvalue_z) (`KismetMathLibrary.BreakVector` (`self.K2_GetActorLocation`)))
  (bind _returnvalue (`self.K2_GetActorLocation`))
  (bind (_startingpoint_x _startingpoint_y) (`KismetMathLibrary.BreakVector` (`self.StartingPoint`)))
  (`parent.ReceiveTick` DeltaSeconds)
  (`self.CheckHealth` (`self.EnemyLife`))
  (if (`|EnumEquality` (`self.AiState`) "NewEnumerator5")
    (set `self.AiState` "NewEnumerator6")
    (`|AIMoveTo` self (`KismetMathLibrary.MakeVector` _startingpoint_x _startingpoint_y _returnvalue_z) null 10.0
      (:`then`
        (if (and (== (`self.K2_GetActorLocation`) (`self.StartingPoint`) :`ErrorTolerance` 5.0) (not (`self.isAtPosition`)))
          (set `self.isAtPosition` true)
          (`GameplayStatics.PlaySoundAtLocation` "/Game/StarterContent/Audio/Collapse_Cue.Collapse_Cue" _returnvalue (struct) 1.0 1.0 0.0 null null null)
          (`KismetSystemLibrary.Delay` 3.0)
          (`/Engine/EditorBlueprintResources/StandardMacros.IncrementInt` (`self.EnemyLife`)
            (:`  `
              (`GameplayStatics.PlaySoundAtLocation` "/Game/Assets/Sounds/heart_coin_sound.heart_coin_sound" _returnvalue (struct) 1.0 1.0 0.0 null null null)
              (`self.SetInitialState`)
              (set `self.isAtPosition` false))))))))

(fn `CheckHealth`
  (params (Lives :type Integer))
  (if (== Lives 1)
    (set `self.AiState` "NewEnumerator5")))

(fn `UserConstructionScript`
  (`parent.UserConstructionScript`))
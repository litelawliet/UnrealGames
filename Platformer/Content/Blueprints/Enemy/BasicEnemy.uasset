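; Basic enemy AI that patrols target actors or roams the navmesh, then chases the player seen through PawnSensing.
; Each behavior sets AiState and runs AIMoveTo: patrol and roam loop, while chase spawns an explosion effect on arrival or falls back to roaming.
; Tick sets walk or run speed by state and destroys the enemy at zero life.
; On collision, the player either attacks it or takes damage and knockback.
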(event `self.PawnSensing.OnSeePawn`
  (params (Pawn :type "Pawn Object Reference"))
  ;[1 1 1] Sense Pawns and follow them
  (`self.Chase Player` Pawn))

(event `Chase Player`
  (params (`Detected Pawn` :type "Pawn Object Reference"))
  (bind _returnvalue (`self.K2_GetActorLocation`))
  ;[1 1 1] Chase Player
  (bind _asthird_person_character (cast `/Game/ThirdPersonBP/Blueprints/ThirdPersonCharacter` `Detected Pawn`))
  (set `self.AiState` "NewEnumerator2")
  (`|AIMoveTo` self (0.0 0.0 0.0) _asthird_person_character
    (:`OnSuccess`
      (`GameplayStatics.SpawnEmitterAtLocation` "/Game/StarterContent/Particles/P_Explosion.P_Explosion" _returnvalue)
      (`GameplayStatics.PlaySoundAtLocation` "/Game/StarterContent/Audio/Explosion_Cue.Explosion_Cue" _returnvalue (struct) 1.0 1.0 0.0 null null null))
    (:`OnFail`
      (`self.Roam`))))

(event `Roam`
  ;[1 1 1] Roam Room
  (set `self.AiState` "NewEnumerator1")
  (`|AIMoveTo` self (`NavigationSystemV1.K2_GetRandomLocationInNavigableRadius` (`self.K2_GetActorLocation`) 1000.0 null null) null
    (:`OnSuccess`
      (`KismetSystemLibrary.Delay` 0.5)
      (`self.Roam`))))

(event `self.ReceiveBeginPlay`
  ;[1 1 1] Start
  (`self.SetInitialState`))

(event `Patrol`
  ;[1 1 1] Patrol
  (set `self.AiState` "NewEnumerator4")
  (`|AIMoveTo` self (0.0 0.0 0.0) (`|GetArrayItem` (`self.Target Position`) (`self.Current Index`))
    (:`OnSuccess`
      _)
    (:`OnFail`
      _))
  (`KismetSystemLibrary.Delay` 1.0)
  (bind _result (`/Engine/EditorBlueprintResources/StandardMacros.IncrementInt` (`self.Current Index`))
    (:`  `
      (if (not (< _result (`KismetArrayLibrary.Array_Length` (`self.Target Position`))))
        (set `self.Current Index` 0))
      (`self.Patrol`))))

(event `self.ReceiveTick`
  (params (DeltaSeconds :type "Float (single-precision)"))
  ;[1 1 1] Update
  (`self.UpdateState`)
  (`self.UpdateLife`))

(event `self.ReceiveHit`
  (params (MyComp :type "PrimitiveComponent Object Reference") (Other :type "Actor Object Reference") (OtherComp :type "PrimitiveComponent Object Reference") (bSelfMoved :type Boolean) (HitLocation :type "Vector Structure") (HitNormal :type "Vector Structure") (NormalImpulse :type "Vector Structure") (Hit :type "HitResult Structure (by ref)"))
  ;[1 1 1] On Colision Hit
  (bind _asthird_person_character (cast `/Game/ThirdPersonBP/Blueprints/ThirdPersonCharacter` Other))
  (bind _hithead (`/Game/ThirdPersonBP/Blueprints/ThirdPersonCharacter.CheckAttackPoint` _asthird_person_character _asthird_person_character))
  (if _hithead
    (`/Game/ThirdPersonBP/Blueprints/ThirdPersonCharacter.AttackEnemy` _asthird_person_character self)
    (else
      (`/Game/ThirdPersonBP/Blueprints/ThirdPersonCharacter.TakeHit` _asthird_person_character 20.0)
      (bind _returnvalue (`self.GetActorForwardVector` _asthird_person_character))
      (bind (_returnvalue_x _returnvalue_y _returnvalue_z) (`KismetMathLibrary.BreakVector` (`KismetMathLibrary.Vector_GetAbs` _returnvalue)))
      (`self.LaunchCharacter` _asthird_person_character (* (* (+ _returnvalue (`KismetMathLibrary.MakeVector` 0.0 0.0 (+ _returnvalue_z 1.0))) (-1.0 -1.0 1.0)) (350.0 350.0 500.0)) true true)
      (set `/Game/ThirdPersonBP/Blueprints/ThirdPersonCharacter.isColliding` false _asthird_person_character))))

(fn `DecrementLife`
  (`/Engine/EditorBlueprintResources/StandardMacros.DecrementInt` (`self.EnemyLife`)))

(fn `SetInitialState`
  (if (`|EnumEquality` (`self.AiState`) "NewEnumerator3")
    _
    (elif (> (`KismetArrayLibrary.Array_Length` (`self.Target Position`)) 0)
      (`self.Patrol`)
      (else
        (`self.Roam`)))))

(fn `UpdateLife`
  (if (<= (`self.EnemyLife`) 0)
    (`self.K2_DestroyActor`)))

(fn `UpdateState`
  (bind _charactermovement (`self.CharacterMovement`))
  (if (`|EnumEquality` (`self.AiState`) "NewEnumerator4")
    (set `CharacterMovementComponent.MaxWalkSpeed` (`self.Walking speed`) _charactermovement)
    (else
      (set `CharacterMovementComponent.MaxWalkSpeed` (`self.Running speed`) _charactermovement))))

(fn `UserConstructionScript`)
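; BankDoor is a Blueprint that raises a referenced Door actor once every actor in its ActorsToKill list is gone.
; It records the door's start position on BeginPlay, then each Tick prunes entries that appear to be empty references from the list.
; Once the list is empty, Tick repeatedly lerps the door toward a fixed height above its start, using the sine of DeltaSeconds as alpha for an eased rise.
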(event `self.ReceiveBeginPlay`
  (set `self.StartPosition` (`self.K2_GetActorLocation` (`self.Door`))))

(event `self.ReceiveTick`
  (params (DeltaSeconds :type "Float (single-precision)"))
  (bind _actorstokill (`self.ActorsToKill`))
  (bind _door (`self.Door`))
  (if (<= (`KismetArrayLibrary.Array_Length` _actorstokill) 0)
    (`self.K2_SetActorLocation` _door (`KismetMathLibrary.VLerp` (`self.K2_GetActorLocation` _door) (+ (`self.StartPosition`) (0.0 0.0 450.0)) (`KismetMathLibrary.Sin` DeltaSeconds)) false false)
    (else
      (for (_array_element _array_index) _actorstokill
        (if (== _array_element null)
          (`KismetArrayLibrary.Array_Remove` _actorstokill _array_index))))))

(fn `UserConstructionScript`)
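; Coin_BP is a collectible gold coin that spins and bobs in place until a player picks it up.
; BeginPlay stores the start location and runs a timeline that offsets it for vertical motion, while Tick adds yaw rotation scaled by delta time.
; On overlap with a ThirdPersonCharacter, it plays a sound at its location, destroys itself and increments that character's CoinsCount.
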(event `self.ReceiveBeginPlay`
  ;[1 1 1] Up and down on Z axis
  (set `self.InitialLocation` (`self.K2_GetActorLocation`))
  (bind (_direction _movement) (`Timeline|Timeline_UpAndDown` :!via `PlayFromStart`)
    (:`Update`
      (`self.K2_SetActorLocation` (+ (`self.InitialLocation`) _movement)))))

(event `self.ReceiveActorBeginOverlap`
  (params (OtherActor :type "Actor Object Reference"))
  ;[1 1 1] Collect coin
  (bind _asthird_person_character (cast `/Game/ThirdPersonBP/Blueprints/ThirdPersonCharacter` OtherActor))
  (`GameplayStatics.PlaySoundAtLocation` (`self.coinSound`) (`self.K2_GetActorLocation`) (struct) 1.0 1.0 0.0 null null null)
  (`self.K2_DestroyActor`)
  (bind _result (`/Engine/EditorBlueprintResources/StandardMacros.IncrementInt` (`/Game/ThirdPersonBP/Blueprints/ThirdPersonCharacter.coinsCount` _asthird_person_character))
    (:`  `
      (set `/Game/ThirdPersonBP/Blueprints/ThirdPersonCharacter.coinsCount` _result _asthird_person_character))))

(event `self.ReceiveTick`
  (params (DeltaSeconds :type "Float (single-precision)"))
  ;[1 1 1] Rotation of the gold coin
  (`self.K2_AddActorLocalRotation` (* (`KismetMathLibrary.MakeRotator` 0.0 0.0 (`self.speedRotation`)) DeltaSeconds)))

(fn `UserConstructionScript`)